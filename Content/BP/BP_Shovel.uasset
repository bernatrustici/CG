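; BP_Shovel is a shovel pickup that advances the player's objective to digging up James Tyrel's body.
; Overlapping its box shows an Interact widget and enables input, but only once the player has found the box; leaving reverses both.
; Pressing E sets FoundShovel on the first-person character, calls GotShovelEvent, updates the objective text, removes the prompt and destroys the actor.
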(event OnComponentBeginOverlap(Box)
  (params (OverlappedComponent :type Primitive%20Component%20Object%20Reference) (OtherActor :type Actor%20Object%20Reference) (OtherComp :type Primitive%20Component%20Object%20Reference) (OtherBodyIndex :type Integer) (bFromSweep :type Boolean) (SweepResult :type Hit%20Result%20Structure%20%28by%20ref%29))
  (bind _returnvalue (Game|GetPlayerController 0))
  ;[1 1 1] doc interactions
  (bind _asbp_first_person_character (Utilities|Casting|CastToBP_FirstPersonCharacter OtherActor))
  (Variables|Default|Setplayer _asbp_first_person_character)
  (if (Variables|/Game/FirstPerson/Blueprints/BP_FirstPersonCharacter.BP_FirstPersonCharacter_C|GetfoundBox (Variables|Default|Getplayer))
    (bind _returnvalue_2 (UserInterface|CreateWidget "/Game/Widget/interact.interact_C" _returnvalue))
    (UserInterface|Viewport|AddtoPlayerScreen _returnvalue_2)
    (Input|EnableInput _returnvalue)))

(event OnComponentEndOverlap(Box)
  (params (OverlappedComponent :type Primitive%20Component%20Object%20Reference) (OtherActor :type Actor%20Object%20Reference) (OtherComp :type Primitive%20Component%20Object%20Reference) (OtherBodyIndex :type Integer))
  ;[1 1 1] doc interactions
  (Utilities|Casting|CastToBP_FirstPersonCharacter OtherActor)
  (if (Variables|/Game/FirstPerson/Blueprints/BP_FirstPersonCharacter.BP_FirstPersonCharacter_C|GetfoundBox (Variables|Default|Getplayer))
    (Input|DisableInput (Game|GetPlayerController 0))
    (Widget|RemovefromParent (stale OnComponentBeginOverlap(Box) _returnvalue_2))))

(event Input|KeyboardEvents|E
  (params (Key :type Key%20Structure :default "None"))
  (bind _player (Variables|Default|Getplayer))
  (bind _player_2 (Variables|Default|Getplayer))
  ;[1 1 1] doc interactions
  (:Pressed
    (if (!= (Variables|/Game/FirstPerson/Blueprints/BP_FirstPersonCharacter.BP_FirstPersonCharacter_C|GetfoundShovel _player) true)
      (Variables|/Game/FirstPerson/Blueprints/BP_FirstPersonCharacter.BP_FirstPersonCharacter_C|SetfoundShovel _player true)
      (Utilities|FlowControl|Sequence
        (:then_0
          (Widget|RemovefromParent (stale OnComponentBeginOverlap(Box) _returnvalue_2))
          (Default|GotShovelEvent _player_2)
          (Variables|/Game/FirstPerson/Blueprints/BP_FirstPersonCharacter.BP_FirstPersonCharacter_C|SetobjActual _player_2 "Dig up James Tyrel's body")
          (Actor|DestroyActor))))))

(fn ConstructionScript)