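; BP_tomb is an interactable tomb that plays a story dialogue and advances the player's objective.
; Its Box overlap enables input and shows an Interact prompt only if the first-person character has GotDocOne.
; Pressing E once locks move and look input, plays Dialogue3, then after a delay updates ObjActual to investigate James Tyrel at administration with a temporary notification.
; The ignore-input calls repeat with true, so this graph never releases that lock.
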(event OnComponentBeginOverlap(Box)
  (params (OverlappedComponent :type Primitive%20Component%20Object%20Reference) (OtherActor :type Actor%20Object%20Reference) (OtherComp :type Primitive%20Component%20Object%20Reference) (OtherBodyIndex :type Integer) (bFromSweep :type Boolean) (SweepResult :type Hit%20Result%20Structure%20%28by%20ref%29))
  (bind _returnvalue (Game|GetPlayerController 0))
  (bind _asbp_first_person_character (Utilities|Casting|CastToBP_FirstPersonCharacter OtherActor))
  (bind _output_get (Variables|Default|Setplayer _asbp_first_person_character))
  (if (Variables|/Game/FirstPerson/Blueprints/BP_FirstPersonCharacter.BP_FirstPersonCharacter_C|GetgotDocOne _output_get)
    (Input|EnableInput _returnvalue)
    (bind _returnvalue_2 (UserInterface|CreateWidget "/Game/Widget/interact.interact_C" _returnvalue))
    (UserInterface|Viewport|AddtoPlayerScreen _returnvalue_2)))

(event OnComponentEndOverlap(Box)
  (params (OverlappedComponent :type Primitive%20Component%20Object%20Reference) (OtherActor :type Actor%20Object%20Reference) (OtherComp :type Primitive%20Component%20Object%20Reference) (OtherBodyIndex :type Integer))
  (Utilities|Casting|CastToBP_FirstPersonCharacter OtherActor)
  (if (Variables|/Game/FirstPerson/Blueprints/BP_FirstPersonCharacter.BP_FirstPersonCharacter_C|GetgotDocOne (stale OnComponentBeginOverlap(Box) _output_get))
    (Input|DisableInput (Game|GetPlayerController 0))
    (Widget|RemovefromParent (stale OnComponentBeginOverlap(Box) _returnvalue_2))))

(event EventBeginPlay)

(event Collision|EventActorBeginOverlap
  (params (OtherActor :type Actor%20Object%20Reference)))

(event EventTick
  (params (DeltaSeconds :type Float%20%28single-precision%29)))

(event Input|KeyboardEvents|E
  (params (Key :type Key%20Structure :default "None"))
  (bind _returnvalue (Game|GetPlayerController 0))
  (bind _returnvalue_2 (Game|GetPlayerController 0))
  (:Pressed
    (Utilities|FlowControl|DoOnce false
      (:Completed
        (Input|SetIgnoreMoveInput _returnvalue_2 true)
        (Input|SetIgnoreLookInput _returnvalue_2 true)
        (Audio|PlaySound2D "/Game/FirstPerson/Audio/dialogue3.dialogue3" 1.0 1.0 0.0 0 0)
        (Input|DisableInput _returnvalue_2)
        (Widget|RemovefromParent (stale OnComponentBeginOverlap(Box) _returnvalue_2))
        (Utilities|FlowControl|Delay 14.0)
        (bind _returnvalue_3 (UserInterface|CreateWidget "/Game/Widget/WB_objUpdated.WB_objUpdated_C"))
        (UserInterface|Viewport|AddtoPlayerScreen _returnvalue_3)
        (Variables|/Game/FirstPerson/Blueprints/BP_FirstPersonCharacter.BP_FirstPersonCharacter_C|SetobjActual (Variables|Default|Getplayer) "Find more information about James Tyrel at administration.")
        (Utilities|FlowControl|Sequence
          (:then_0
            (Utilities|FlowControl|Delay 5.0)
            (Widget|RemovefromParent _returnvalue_3))
          (:then_1
            (Input|SetIgnoreMoveInput _returnvalue true)
            (Input|SetIgnoreLookInput _returnvalue true)))))))

(fn ConstructionScript)